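; BP_FastInputManager customizes the selection list that a fast-input helper offers for a named property.
; GetCustomSelections constructs a second manager, copies the property context into it, then clears its own custom selections.
; For the Tags property, it retargets that helper to ComponentTags, reads JSON, builds selections and appends the helper's Selections, so Tags reuses the ComponentTags choices.
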(fn `GetCustomSelections`
  (locals (FastInputHelper :type "/Game/BP_FastInputManager Object Reference"))
  (bind _returnvalue (`|GenericCreateObject` "BP_FastInputManager_C"))
  (set `local.FastInputHelper` _returnvalue)
  (`|ExecutionSequence`
    (:`then_0`
      ;[1 1 1] 先同步一下数据
      (set `FastInputManager.PropertyName` (`self.PropertyName`) (`local.FastInputHelper`))
      (set `FastInputManager.PropertyOwnerStruct` (`self.PropertyOwnerStruct`) (`local.FastInputHelper`))
      (set `FastInputManager.PropertyActorClass` (`self.PropertyActorClass`) (`local.FastInputHelper`)))
    (:`then_1`
      (`KismetArrayLibrary.Array_Clear` (`self.CustomSelections`))
      (switch `string` (`self.PropertyName`)
        (:`Tags`
          (set `FastInputManager.PropertyName` "ComponentTags" (`local.FastInputHelper`))
          (`self.FIReadJson` (`local.FastInputHelper`))
          (`self.GetSelections` (`local.FastInputHelper`))
          (`self.GetCustomSelections` (`local.FastInputHelper`))
          (`KismetArrayLibrary.Array_Append` (`self.CustomSelections`) (`FastInputManager.Selections` (`local.FastInputHelper`)))
          (return))))))